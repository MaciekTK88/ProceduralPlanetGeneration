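; Planet spawner actor that regenerates a chunk-based planet, with support for ticking in the editor.
; RegeneratePlanet stops tick, resets state flags, clears components, precomputes chunk data and recompiles the Planet compute shader.
; If SafetyCheck passes, it flags generation as allowed and re-enables tick in editor mode.
; The construction script sets console variables that disable fast sky atmosphere LUTs and force directional virtual shadow cache invalidation.
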(event `self.ReceiveBeginPlay`)

(event `RegeneratePlanet`
  (`self.SetActorTickEnabled` false)
  (set `self.SaveToGenerate` false)
  (set `self.ready` false)
  (`self.ClearComponents`)
  (`self.PrecomputeChunkData`)
  (`KismetSystemLibrary.ExecuteConsoleCommand` "RecompileShaders /ComputeShaderShaders/Planet.usf" null)
  (bind _returnvalue (`self.SafetyCheck`))
  (if _returnvalue
    (set `self.SaveToGenerate` true)
    (set `self.UseEditorTick` true)
    (`self.SetActorTickEnabled` true)))

(fn `UserConstructionScript`
  (`KismetSystemLibrary.ExecuteConsoleCommand` "r.SkyAtmosphere.AerialPerspectiveLUT.FastApplyOnOpaque 0" null)
  (`KismetSystemLibrary.ExecuteConsoleCommand` "r.SkyAtmosphere.FastSkyLUT 0" null)
  (`KismetSystemLibrary.ExecuteConsoleCommand` "r.Shadow.Virtual.Cache.ForceInvalidateDirectional 1" null))